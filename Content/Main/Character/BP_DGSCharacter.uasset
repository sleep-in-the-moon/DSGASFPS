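; Character Blueprint that starts play with BP_Rifle equipped through SpawnNewWeaponAndEquip, with debug keys to switch between unarmed and rifle.
; A separate SwitchGun event flip-flops linked anim layers on the mesh.
; Its rifle branch plays the equip montage, then after a delay attaches a new rifle mesh component to a hand socket, with no removal on the unarmed branch.
; Velocity and acceleration debug-arrow nodes are disconnected.
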(event Custom|SwitchGun
  (bind _mesh (Variables|Character|GetMesh))
  (Utilities|FlowControl|FlipFlop
    (:A
      (Components|SkeletalMesh|AnimationBlueprintLinking|LinkAnimClassLayers (Variables|Character|GetMesh) "/Game/Main/Character/ABP_UnarmAnimLayer.ABP_UnarmAnimLayer_C"))
    (:B
      (Animation|Montage|PlayMontage _mesh "/Game/Main/Character/Anim/Actions/Montage/MM_Rifle_Equip_Montage.MM_Rifle_Equip_Montage"
        (:then
          (Components|SkeletalMesh|AnimationBlueprintLinking|LinkAnimClassLayers _mesh "/Game/Main/Character/ABP_RifleAnimLayer.ABP_RifleAnimLayer_C")
          (Utilities|FlowControl|Delay 0.42)
          (bind _returnvalue (AddComponent|AddSkeletalMeshComponent false))
          (Collision|SetCollisionEnabled _returnvalue "NoCollision")
          (Components|SkeletalMesh|SetSkeletalMeshAsset _returnvalue "/Game/Weapons/Rifle/Mesh/SK_Rifle.SK_Rifle")
          (Transformation|AttachComponentToComponent _returnvalue (Variables|Character|GetMesh) "weapon_r_muzzle" "KeepWorld" "KeepRelative" "KeepRelative" false)
          (Transformation|SetRelativeTransform _returnvalue (Math|Transform|MakeTransform "-45.000000,0.000000,-25.000000" "0.000000,-90.000000,0.000000") false false))))))

(event EventBeginPlay
  (Class|DGSBasicCharacter|SpawnNewWeaponandEquip "/Game/Main/Weapon/BP_Rifle.BP_Rifle_C"))

(event EventTick
  (params (DeltaSeconds :type Float%20%28single-precision%29)))

(event Input|KeyboardEvents|DebugKey1
  (params (Key :type Key%20Structure :default "None") (ActionValue :type Input%20Action%20Value%20Structure))
  (:Pressed
    (Class|DGSBasicCharacter|SpawnNewWeaponandEquip "/Game/Main/Weapon/BP_Rifle.BP_Rifle_C")))

(event Input|KeyboardEvents|DebugKey0
  (params (Key :type Key%20Structure :default "None") (ActionValue :type Input%20Action%20Value%20Structure))
  (:Pressed
    (Class|DGSBasicCharacter|SpawnNewWeaponandEquip "/Game/Main/Weapon/BP_Unarmed.BP_Unarmed_C")))

(fn ConstructionScript)